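; BP_Demo_Input_Simulator is a demo actor that plays a scripted input sequence on third-person characters inside its Box.
; Starting shortly after BeginPlay, it injects each step through Enhanced Input's continuous injection on the overlapping characters' player controllers.
; A timer governs each step's duration, with an interval between steps and optional looping.
; Leaving the Box stops the current injected input for that player.
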(event OnComponentEndOverlap(Box)
  (params (OverlappedComponent :type Primitive%20Component%20Object%20Reference) (OtherActor :type Actor%20Object%20Reference) (OtherComp :type Primitive%20Component%20Object%20Reference) (OtherBodyIndex :type Integer))
  (bind _asplayer_controller (Utilities|Casting|CastToPlayerController (Game|GetInstigatorController OtherActor)))
  (Class|EnhancedInputSubsystemInterface|StopContinuousInputInjectionforAction(Message) (PlayerController|LocalPlayerSubsystems|GetEnhancedInputLocalPlayerSubsystem _asplayer_controller) (.input (Utilities|Array|Get(acopy) (Variables|Default|GetInput%20Sequence) (Variables|Default|GetCurrent%20Index)))))

(event Custom|Start%20Sequence
  (Variables|Default|SetCurrent%20Index 0)
  (CallFunction|ApplyAction))

(event Custom|Stop%20Input
  (for _array_element (CallFunction|GetSystems)
    (Class|EnhancedInputSubsystemInterface|StopContinuousInputInjectionforAction(Message) (PlayerController|LocalPlayerSubsystems|GetEnhancedInputLocalPlayerSubsystem _array_element) (.input (Utilities|Array|Get(acopy) (Variables|Default|GetInput%20Sequence) (Variables|Default|GetCurrent%20Index)))))
  (bind _result (Math|Integer|IncrementInt (Variables|Default|GetCurrent%20Index))
    (:%20%20
      (if (> _result (Utilities|Array|LastIndex (Variables|Default|GetInput%20Sequence)))
        (Variables|Default|SetCurrent%20Index 0)
        (if (Variables|Default|GetLoop)
          (Utilities|FlowControl|Delay (Variables|Default|GetSequence%20Intervals) :!label _label)
          (CallFunction|ApplyAction))
        (else
          (goto _label))))))

(event Custom|Apply%20Action
  (bind _input_sequence (Variables|Default|GetInput%20Sequence))
  (bind _current_index (Variables|Default|GetCurrent%20Index))
  (bind _output (Utilities|Array|Get(acopy) _input_sequence _current_index))
  (for _array_element (CallFunction|GetSystems)
    (Class|EnhancedInputSubsystemInterface|StartContinuousInputInjectionforAction(Message) (PlayerController|LocalPlayerSubsystems|GetEnhancedInputLocalPlayerSubsystem _array_element) (.input _output) (Utilities|Struct|MakeInputActionValue (.x (.vectorvalue _output)) (.y (.vectorvalue _output)) (.z (.vectorvalue _output)) "Boolean") (.modifier _output)))
  (Utilities|Time|SetTimerbyEvent (EventDispatchers|CreateEvent :!event Custom|Stop%20Input) (.duration _output)))

(event EventBeginPlay
  (Utilities|FlowControl|Delay 1.0)
  (CallFunction|StartSequence))

(fn ConstructionScript
  (Transformation|SetRelativeLocation (Variables|Default|GetBox) (Variables|Default|GetNew%20Location) false false))

(fn GetSystems
  (bind _newlocalvar_0 (LocalVariables|GetNewLocalVar_0))
  (for _array_element (Collision|GetOverlappingActors (Variables|Default|GetBox) "/Game/Project_Modular_GBS/Blueprints/Player/BP_ThirdPersonCharacter.BP_ThirdPersonCharacter_C" :!class /Script/Engine.PrimitiveComponent)
    (bind _asplayer_controller (Utilities|Casting|CastToPlayerController (Game|GetInstigatorController _array_element)))
    (Utilities|Array|Add _newlocalvar_0 _asplayer_controller))
  (return _newlocalvar_0))