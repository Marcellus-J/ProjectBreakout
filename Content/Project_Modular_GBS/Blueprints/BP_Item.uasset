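; BP_Item is a pickup item actor that takes its mesh, material, pickup radius and owner/external interactions from an ItemData asset at construction.
; It records the pawn that picks it up as Instigator and lazily creates a W_Item widget to display it.
; Quantity changes refresh the widget or destroy non-infinite items at zero.
; On destruction or world removal it removes the widget, unequips if right-hand held, and leaves the Instigator's container.
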(event EventPickedUp
  (params (Actor%20Ref :type Actor%20Object%20Reference))
  (bind _aspawn (Utilities|Casting|CastToPawn Actor%20Ref))
  (Variables|Actor|SetInstigator _aspawn))

(event EventItemQuantityUpdated
  (if (not (Variables|/Game/Project_Modular_GBS/Blueprints/Systems/Systems_Setup/DA_Item.DA_Item_C|GetInfinit (Variables|Default|GetItem%20Data)))
    (if (<= (Variables|Default|GetQuantity) 0)
      (Actor|DestroyActor)
      (else
        (CallFunction|UpdateWidget)))))

(event EventUpdateWidget
  (Class|BPIItem|UpdateLable(Message) (Variables|Default|GetItem%20Widget)))

(event EventEquipItem
  (Class|BPIInteract|ShowAllInteractions(Message) (Actor|GetComponentbyClass (Variables|Actor|GetInstigator) "/Game/Project_Modular_GBS/Blueprints/Systems/Interaction_System.Interaction_System_C") self true))

(event EventEndPlay
  (params (EndPlayReason :type EEndPlayReason%20Enum :default "Destroyed"))
  (switch Utilities|FlowControl|Switch|SwitchonEEndPlayReason EndPlayReason
    (:Destroyed
      _)
    (:RemovedFromWorld
      _))
  (CallFunction|BeforeDestoy))

(fn ConstructionScript
  (Variables|Default|GetItem%20Data
    (:then
      (CallFunction|InnitItemData)
      (CallFunction|InnitInteractions)
      (if (Variables|Default|GetStart%20With%20Max%20Stack)
        (Variables|Default|SetQuantity (Variables|/Game/Project_Modular_GBS/Blueprints/Systems/Systems_Setup/DA_Item.DA_Item_C|GetMax%20Per%20Stack (Variables|Default|GetItem%20Data)))))
    (:else)))

(fn InnitItemData
  (bind _static_mesh (Variables|Default|GetStatic%20Mesh))
  (bind _item_data (Variables|Default|GetItem%20Data))
  (Components|StaticMesh|SetStaticMesh _static_mesh (Variables|/Game/Project_Modular_GBS/Blueprints/Systems/Systems_Setup/DA_Item.DA_Item_C|GetModel _item_data))
  (bind _material (Variables|/Game/Project_Modular_GBS/Blueprints/Systems/Systems_Setup/DA_Item.DA_Item_C|GetMaterial _item_data)
    (:then
      (Rendering|Material|SetMaterial _static_mesh 0 _material))
    (:else
      _))
  (Components|Sphere|SetSphereRadius (Variables|Default|GetPickUp%20Collision) (Variables|/Game/Project_Modular_GBS/Blueprints/Systems/Systems_Setup/DA_Item.DA_Item_C|GetPick%20UP%20Radius _item_data) true)
  (return))

(fn GetWidget
  (bind _item_widget (Variables|Default|GetItem%20Widget)
    (:then
      (return _item_widget))
    (:else
      (bind _returnvalue (UserInterface|CreateWidget "/Game/Project_Modular_GBS/Default_Demo_Widgets/W_Item.W_Item_C" 0 self))
      (bind _output_get (Variables|Default|SetItem%20Widget _returnvalue))
      (return _output_get))))

(fn InnitInteractions
  (bind _returnvalue (Actor|GetComponentbyClass "/Game/Project_Modular_GBS/Blueprints/Systems/Interaction_System.Interaction_System_C"))
  (bind _item_data (Variables|Default|GetItem%20Data))
  (Utilities|IsValid _returnvalue
    (:Is%20Valid
      (bind _output_get (LocalVariables|SetInteraction%20System%20Ref _returnvalue))
      (Default|UpdateInteractions _output_get (Variables|/Game/Project_Modular_GBS/Blueprints/Systems/Systems_Setup/DA_Item.DA_Item_C|GetOwner%20Actions _item_data) (Variables|/Game/Project_Modular_GBS/Blueprints/Systems/Systems_Setup/DA_Item.DA_Item_C|GetExternal%20Actions _item_data)))))

(fn QueryActions
  (return 0 0))

(fn BeforeDestoy
  (bind _self self)
  (bind _instigator (Variables|Actor|GetInstigator)
    (:then
      (Widget|RemovefromParent (Variables|Default|GetItem%20Widget))
      (Utilities|FlowControl|Sequence
        (:then_0
          (Utilities|IsValid (Actor|GetComponentbyClass _instigator "/Game/Project_Modular_GBS/Blueprints/Systems/Equip_System.Equip_System_C")
            (:Is%20Valid
              (if (== (Variables|/Game/Project_Modular_GBS/Blueprints/Systems/Equip_System.Equip_System_C|GetCurrent%20RH%20Item (Actor|GetComponentbyClass _instigator "/Game/Project_Modular_GBS/Blueprints/Systems/Equip_System.Equip_System_C")) _self)
                (Default|UnEquipAll (Actor|GetComponentbyClass _instigator "/Game/Project_Modular_GBS/Blueprints/Systems/Equip_System.Equip_System_C"))))))
        (:then_1
          (Class|BPIContainer|TryRemoveItem(Message) (Actor|GetComponentbyClass _instigator "/Game/Project_Modular_GBS/Blueprints/Systems/Container_System.Container_System_C") _self))))
    (:else)))