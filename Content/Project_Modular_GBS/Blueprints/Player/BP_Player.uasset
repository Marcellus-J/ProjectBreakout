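; BP_Player is the player Blueprint, which handles interaction with actors in the world.
; While interaction is enabled, each tick runs a TraceSystem ranged trace from center to show or hide InteractionSystem messages for the hit actor.
; Possessing and unpossessing toggle this check.
; Separately, capsule overlaps trigger InteractionSystem interaction when auto pickup is on.
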(event OnComponentBeginOverlap(CapsuleComponent)
  (params (OverlappedComponent :type Primitive%20Component%20Object%20Reference) (OtherActor :type Actor%20Object%20Reference) (OtherComp :type Primitive%20Component%20Object%20Reference) (OtherBodyIndex :type Integer) (bFromSweep :type Boolean) (SweepResult :type Hit%20Result%20Structure%20%28by%20ref%29))
  (if (Variables|Default|GetAuto%20PickUp)
    (Default|Interact (Variables|Default|GetInteraction_System) self OtherActor)))

(event Custom|Enable%20Player%20Interaction
  (params (Enable :type Boolean))
  (Variables|Default|SetPlayer%20Interaction Enable))

(event EventPossessed
  (params (NewController :type Controller%20Object%20Reference))
  (CallFunction|EnablePlayerInteraction true))

(event EventTick
  (params (DeltaSeconds :type Float%20%28single-precision%29))
  (CallFunction|CallPlayerInteraction))

(event EventUnpossessed
  (params (OldController :type Controller%20Object%20Reference))
  (CallFunction|EnablePlayerInteraction false))

(fn ConstructionScript
  (|CallParentFunction))

(fn QueryActions
  (return 0 0))

(fn CallPlayerInteraction
  (bind _interaction_system (Variables|Default|GetInteraction_System))
  (if (Variables|Default|GetPlayer%20Interaction)
    (bind (_hit_any _hit) (Default|FromCenterRanged (Variables|Default|GetTrace_System) "NewEnumerator1" false false 0.0))
    (if _hit_any
      (Class|BPIInteract|ShowAllInteractions(Message) _interaction_system (.HitActor (Collision|BreakHitResult _hit)) false)
      (else
        (Class|BPIInteract|HideAllInteractions(Message) _interaction_system false)))))