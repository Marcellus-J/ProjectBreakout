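; BP_Firing_Demo_Weapon is a demo actor for switching the data used by its FiringSystem between two weapon setups.
; Two sphere components act as overlap triggers: Sphere2 applies Rifle and Sphere1 applies Burst_Rifle through UpdateSystemData.
; Both overlaps then write the current FiringData to a TextRender as a readout, with no filter on the overlapping actor.
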(event OnComponentBeginOverlap(Sphere2)
  (params (OverlappedComponent :type Primitive%20Component%20Object%20Reference) (OtherActor :type Actor%20Object%20Reference) (OtherComp :type Primitive%20Component%20Object%20Reference) (OtherBodyIndex :type Integer) (bFromSweep :type Boolean) (SweepResult :type Hit%20Result%20Structure%20%28by%20ref%29))
  (bind _firing_system (Variables|Default|GetFiring_System))
  (Default|UpdateSystemData _firing_system "/Game/Project_Modular_GBS/Items_DataBase/Weapons_Data/Rifle.Rifle")
  (Rendering|Components|TextRender|SetText (Variables|Default|GetTextRender) (Utilities|Text|ToText(Object) (Variables|/Game/Project_Modular_GBS/Blueprints/Systems/Firing_System.Firing_System_C|GetFiring_Data _firing_system))))

(event OnComponentBeginOverlap(Sphere1)
  (params (OverlappedComponent :type Primitive%20Component%20Object%20Reference) (OtherActor :type Actor%20Object%20Reference) (OtherComp :type Primitive%20Component%20Object%20Reference) (OtherBodyIndex :type Integer) (bFromSweep :type Boolean) (SweepResult :type Hit%20Result%20Structure%20%28by%20ref%29))
  (Default|UpdateSystemData (Variables|Default|GetFiring_System) "/Game/Project_Modular_GBS/Items_DataBase/Weapons_Data/Burst_Rifle.Burst_Rifle")
  (Rendering|Components|TextRender|SetText (Variables|Default|GetTextRender) (Utilities|Text|ToText(Object) (Variables|/Game/Project_Modular_GBS/Blueprints/Systems/Firing_System.Firing_System_C|GetFiring_Data (Variables|Default|GetFiring_System)))))

(fn ConstructionScript
  (|CallParentFunction))