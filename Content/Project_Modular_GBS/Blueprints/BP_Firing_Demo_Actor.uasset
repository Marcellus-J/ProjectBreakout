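; Demo actor that exercises the modular firing and trace components, shooting automatically while something overlaps its sphere.
; Overlap begin and end open and close a Tick gate after a short retriggerable delay, so Fire is attempted every frame.
; Each shot the FiringSystem accepts runs a TraceSystem trace with angular inaccuracy toward TraceEnd and refreshes the ammo text.
; The construction script positions TraceEnd from TraceTarget.
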(event OnComponentEndOverlap(Sphere)
  (params (OverlappedComponent :type Primitive%20Component%20Object%20Reference) (OtherActor :type Actor%20Object%20Reference) (OtherComp :type Primitive%20Component%20Object%20Reference) (OtherBodyIndex :type Integer))
  (Utilities|FlowControl|RetriggerableDelay 0.1)
  (CallFunction|StopFire))

(event OnComponentBeginOverlap(Sphere)
  (params (OverlappedComponent :type Primitive%20Component%20Object%20Reference) (OtherActor :type Actor%20Object%20Reference) (OtherComp :type Primitive%20Component%20Object%20Reference) (OtherBodyIndex :type Integer) (bFromSweep :type Boolean) (SweepResult :type Hit%20Result%20Structure%20%28by%20ref%29))
  (Utilities|FlowControl|RetriggerableDelay 0.1)
  (CallFunction|StartFire))

(event Custom|Fire
  (bind _fired (Class|BPIFiring|TryFire(Message) (Variables|Default|GetFiring_System)))
  (if _fired
    (Default|FromAtoB (Variables|Default|GetTrace_System) (Transformation|GetWorldLocation (Variables|Default|GetDefaultSceneRoot)) (Transformation|GetWorldLocation (Variables|Default|GetTrace%20End)) 2e+01 true)
    (Rendering|Components|TextRender|SetText (Variables|Default|GetTextRender) (Utilities|Text|FormatText "Ammo: {1}" (Utilities|Text|ToText(Integer) (Variables|/Game/Project_Modular_GBS/Blueprints/Systems/Firing_System.Firing_System_C|GetCurrent%20Ammo (Variables|Default|GetFiring_System)))))))

(event Custom|Start%20Fire
  (Utilities|FlowControl|Gate true) ; enters at Open
)

(event Custom|Stop%20Fire
  (Class|BPIFiring|TryStopFire(Message) (Variables|Default|GetFiring_System))
  (Utilities|FlowControl|Gate true) ; enters at Close
)

(event EventBeginPlay
  (Rendering|Components|TextRender|SetText (Variables|Default|GetTextRender) (Utilities|Text|FormatText "Ammo: {1}" (Utilities|Text|ToText(Integer) (Variables|/Game/Project_Modular_GBS/Blueprints/Systems/Firing_System.Firing_System_C|GetCurrent%20Ammo (Variables|Default|GetFiring_System))))))

(event EventTick
  (params (DeltaSeconds :type Float%20%28single-precision%29))
  (Utilities|FlowControl|Gate true
    (:Exit
      (CallFunction|Fire))))

(fn ConstructionScript
  (Transformation|SetRelativeLocation (Variables|Default|GetTrace%20End) (Variables|Default|GetTrace%20Target) false false))