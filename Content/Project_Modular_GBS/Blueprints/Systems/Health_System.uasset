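; Health system component that applies stat changes to its owner and coordinates them with an optional Shield_System on the same actor.
; For the combined target stat, additions fill health first and spill into shield, while removals drain shield first and spill into health, using TryAdjust's out-of-range remainder.
; Other targets, or owners without a shield, adjust health alone.
; Every AdjustStatus event then attempts regeneration.
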(event EventAdjustStatus
  (params (Target%20Stat :type E_Status%20Enum :default "NewEnumerator3") (Add/Remove :type Boolean) (Value :type Float%20%28double-precision%29) (Max%20Value :type Float%20%28double-precision%29) (Causer :type Actor%20Object%20Reference))
  (CallFunction|AdjustBoth Target%20Stat Add/Remove Value)
  (CallFunction|TryRegeneration))

(fn AdjustBoth
  (params (Target%20Stat :type E_Status%20Enum :default "NewEnumerator3") (Add/Remove :type Boolean) (Value :type Float%20%28double-precision%29))
  (bind _returnvalue (Components|GetOwner))
  (bind _returnvalue_2 (Actor|GetComponentbyClass _returnvalue "/Game/Project_Modular_GBS/Blueprints/Systems/Shield_System.Shield_System_C"))
  (if (Utilities|Enum|Equal(Enum) Target%20Stat "NewEnumerator4")
    (Utilities|IsValid _returnvalue_2
      (:Is%20Valid
        (LocalVariables|SetShield%20System _returnvalue_2)
        (if Add/Remove
          (bind (_out_of_range _amount) (CallFunction|TryAdjust Add/Remove Value))
          (if _out_of_range
            (Default|TryAdjust (LocalVariables|GetShield%20System) Add/Remove _amount))
          (else
            (bind (_out_of_range_2 _amount_2) (Default|TryAdjust (LocalVariables|GetShield%20System) Add/Remove Value))
            (if _out_of_range_2
              (CallFunction|TryAdjust Add/Remove _amount_2)))))
      (:Is%20Not%20Valid
        (CallFunction|TryAdjust Add/Remove Value :!label _label)))
    (else
      (goto _label))))