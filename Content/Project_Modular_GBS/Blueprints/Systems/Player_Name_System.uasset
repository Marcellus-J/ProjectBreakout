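; Player name component that shows a floating name tag on its owning actor.
; On BeginPlay it adds a non-colliding, screen-space widget component to the owner, offset slightly above RelativeLocation and sized to the widget's desired size.
; It creates W_Player_Name with a reference to itself, then fills in the text from the data message on player state index 0, rather than one looked up from the owner.
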(event EventBeginPlay
  (bind _relativelocation (Variables|Default|GetRelativeLocation))
  (bind _returnvalue (Game|AddComponentbyClass (Components|GetOwner) "/Script/UMG.WidgetComponent" false (Math|Transform|MakeTransform (Math|Vector|MakeVector (.x _relativelocation) (.y _relativelocation) (+ (.z _relativelocation) 3e+01)) "0, 0, 0" "1.000000,1.000000,1.000000")))
  (Rendering|Material|SetMaterial _returnvalue 0 "/Game/Project_Modular_GBS/Materials/MI_Player_Name.MI_Player_Name")
  (Collision|SetCollisionEnabled _returnvalue "NoCollision")
  (Class|WidgetComponent|SetDrawatDesiredSize _returnvalue true)
  (Class|WidgetComponent|SetWidgetSpace _returnvalue "Screen")
  (bind _returnvalue_2 (UserInterface|CreateWidget "/Game/Project_Modular_GBS/Default_Demo_Widgets/W_Player_Name.W_Player_Name_C" 0 self))
  (bind _output_get (Variables|Default|SetWidget%20Ref _returnvalue_2))
  (UserInterface|SetWidget _returnvalue _output_get)
  (bind _player_name (Class|BPIPlayerState|GetData(Message) (Game|GetPlayerState 0)))
  (Default|UpdatePlayerName _output_get (Utilities|Text|ToText(Name) _player_name)))