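; Damage_System provides Damage and Heal functions that apply stat changes to a targeted actor.
; Each selects the actor's Health_System or Shield_System component by DamageTarget, with HealthAndShield preferring Health and falling back to Shield.
; The selected component receives AdjustStatusMessage with the target stat, value and causer, and Heal sets AddRemove to true.
; Custom and Stamina targets have no component wired.
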(fn Damage
  (params (Targeted%20Actor :type Actor%20Object%20Reference) (Damage%20Target :type E_Status%20Enum :default "NewEnumerator3") (Value :type Float%20%28double-precision%29) (Causer :type Actor%20Object%20Reference))
  (bind _returnvalue (Actor|GetComponentbyClass Targeted%20Actor "/Game/Project_Modular_GBS/Blueprints/Systems/Health_System.Health_System_C"))
  (bind _returnvalue_2 (Actor|GetComponentbyClass Targeted%20Actor "/Game/Project_Modular_GBS/Blueprints/Systems/Shield_System.Shield_System_C"))
  (Class|BPIStatus|AdjustStatus(Message) (Utilities|Select :Index Damage%20Target :NewEnumerator3 0 :NewEnumerator0 _returnvalue :NewEnumerator1 _returnvalue_2 :NewEnumerator4 (select (Utilities|IsValid _returnvalue) _returnvalue _returnvalue_2) :NewEnumerator5 0) Damage%20Target false Value 0.0 Causer))

(fn Heal
  (params (Targeted%20Actor :type Actor%20Object%20Reference) (Damage%20Target :type E_Status%20Enum :default "NewEnumerator3") (Value :type Float%20%28double-precision%29) (Causer :type Actor%20Object%20Reference))
  (bind _returnvalue (Actor|GetComponentbyClass Targeted%20Actor "/Game/Project_Modular_GBS/Blueprints/Systems/Health_System.Health_System_C"))
  (bind _returnvalue_2 (Actor|GetComponentbyClass Targeted%20Actor "/Game/Project_Modular_GBS/Blueprints/Systems/Shield_System.Shield_System_C"))
  (Class|BPIStatus|AdjustStatus(Message) (Utilities|Select :Index Damage%20Target :NewEnumerator3 0 :NewEnumerator0 _returnvalue :NewEnumerator1 _returnvalue_2 :NewEnumerator4 (select (Utilities|IsValid _returnvalue) _returnvalue _returnvalue_2) :NewEnumerator5 0) Damage%20Target true Value 0.0 Causer))