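; Equip system that lets its owner equip items from a container into the right hand through five hotkeys and an unequip input.
; EquipItem finds the owner's Container_System of the target type, unequips the current item, then looks up the slot by index.
; Equipping and unequipping notify the item and the character mesh's anim instance through messages, passing the item type to drive animation.
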(event Input|EnhancedActionEvents|EnhancedInputActionIA_Equip_1
  (params (ActionValue :type Vector%202D%20Structure) (ElapsedSeconds :type Float%20%28double-precision%29) (TriggeredSeconds :type Float%20%28double-precision%29) (InputAction :type Input%20Action%20Object%20Reference :default "/Game/Project_Modular_GBS/Blueprints/Player/Input/IA_Equip_1.IA_Equip_1"))
  (:Started
    (CallFunction|EquipItem 0 "NewEnumerator0")))

(event Input|EnhancedActionEvents|EnhancedInputActionIA_Equip_4
  (params (ActionValue :type Boolean) (ElapsedSeconds :type Float%20%28double-precision%29) (TriggeredSeconds :type Float%20%28double-precision%29) (InputAction :type Input%20Action%20Object%20Reference :default "/Game/Project_Modular_GBS/Blueprints/Player/Input/IA_Equip_4.IA_Equip_4"))
  (:Started
    (CallFunction|EquipItem 3 "NewEnumerator0")))

(event Input|EnhancedActionEvents|EnhancedInputActionIA_Equip_2
  (params (ActionValue :type Boolean) (ElapsedSeconds :type Float%20%28double-precision%29) (TriggeredSeconds :type Float%20%28double-precision%29) (InputAction :type Input%20Action%20Object%20Reference :default "/Game/Project_Modular_GBS/Blueprints/Player/Input/IA_Equip_2.IA_Equip_2"))
  (:Started
    (CallFunction|EquipItem 1 "NewEnumerator0")))

(event Input|EnhancedActionEvents|EnhancedInputActionIA_Equip_3
  (params (ActionValue :type Boolean) (ElapsedSeconds :type Float%20%28double-precision%29) (TriggeredSeconds :type Float%20%28double-precision%29) (InputAction :type Input%20Action%20Object%20Reference :default "/Game/Project_Modular_GBS/Blueprints/Player/Input/IA_Equip_3.IA_Equip_3"))
  (:Started
    (CallFunction|EquipItem 2 "NewEnumerator0")))

(event Input|EnhancedActionEvents|EnhancedInputActionIA_UnEquip
  (params (ActionValue :type Vector%202D%20Structure) (ElapsedSeconds :type Float%20%28double-precision%29) (TriggeredSeconds :type Float%20%28double-precision%29) (InputAction :type Input%20Action%20Object%20Reference :default "/Game/Project_Modular_GBS/Blueprints/Player/Input/IA_UnEquip.IA_UnEquip"))
  (:Started
    (CallFunction|UnEquipAll)))

(event Input|EnhancedActionEvents|EnhancedInputActionIA_Equip_5
  (params (ActionValue :type Boolean) (ElapsedSeconds :type Float%20%28double-precision%29) (TriggeredSeconds :type Float%20%28double-precision%29) (InputAction :type Input%20Action%20Object%20Reference :default "/Game/Project_Modular_GBS/Blueprints/Player/Input/IA_Equip_5.IA_Equip_5"))
  (:Started
    (CallFunction|EquipItem 4 "NewEnumerator0")))

(fn EquipItem
  (params (Item%20Index :type Integer) (Target%20Container :type E_Container_Type%20Enum :default "NewEnumerator0"))
  (for _array_element (Actor|GetComponentsByClass (Components|GetOwner) "/Game/Project_Modular_GBS/Blueprints/Systems/Container_System.Container_System_C")
    (if (Utilities|Enum|Equal(Enum) (Variables|/Game/Project_Modular_GBS/Blueprints/Systems/Container_System.Container_System_C|GetContainer%20Type _array_element) Target%20Container)
      (CallFunction|UnEquipAll)
      (if (.Found (Default|QueryContainerbyIndex _array_element Item%20Index))
        (bind _output_get (Variables|Default|SetCurrent%20RH%20Item (.Item%20Ref (Default|QueryContainerbyIndex _array_element Item%20Index))))
        (Class|BPIAnimations|EquippedItemType(Message) (.Anim%20Instance%20Ref (CallFunction|GetAnimInstance)) (Variables|/Game/Project_Modular_GBS/Blueprints/Systems/Systems_Setup/DA_Item.DA_Item_C|GetItem%20Type (Variables|/Game/Project_Modular_GBS/Blueprints/BP_Item.BP_Item_C|GetItem%20Data _output_get)))
        (Class|BPIItem|EquipItem(Message) _output_get)
        (return true)
        (else
          (return false)))))
  (return false))

(fn UnEquipAll
  (Class|BPIItem|UnEquipItem(Message) (Variables|Default|GetCurrent%20RH%20Item))
  (Variables|Default|SetCurrent%20RH%20Item 0)
  (Class|BPIAnimations|EquippedItemType(Message) (.Anim%20Instance%20Ref (CallFunction|GetAnimInstance)) "NewEnumerator3"))

(fn GetAnimInstance
  (bind _ascharacter (Utilities|Casting|CastToCharacter (Components|GetOwner))
    (:then
      (return true (Components|SkeletalMesh|GetAnimInstance (Variables|/Script/Engine.Character|GetMesh _ascharacter))))
    (:CastFailed
      (return false 0))))