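; Modular movement component that binds Enhanced Input to its owning Character for move, look, jump, crouch, run, aim and fire.
; Aiming or firing switches rotation to controller-facing and notifies the AnimInstance, with a retriggerable delay before firing ends.
; Adjust events alter speed, gravity and carried weight, then TakeEffect reapplies walk speed and gravity scale using a weight multiplier.
; Run sets walk speed directly, bypassing those multipliers.
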(event Custom|Update_View
  (params (scale :type Vector%202D%20Structure))
  (bind _returnvalue (Game|Player|GetPlayerPawn 0))
  (bind _mouse_sensetivity (Variables|Default|GetMouse%20Sensetivity))
  (bind _returnvalue_2 (* scale _mouse_sensetivity))
  (bind (_x _y) (Math|Vector2D|BreakVector2D _returnvalue_2))
  ;[1 1 1] Comment
  (Pawn|Input|AddControllerYawInput _returnvalue _x)
  (Pawn|Input|AddControllerPitchInput _returnvalue _y))

(event Custom|Take%20Effect
  (bind _multiplier (Utilities|GetWeightMultiplier))
  (bind _movement_comp_ref (Variables|Default|GetMovement%20Comp%20Ref))
  ;[1 1 1] Comment
  ;;[1 1 1] Comment
  (Variables|/Script/Engine.CharacterMovementComponent|SetGravityScale _movement_comp_ref (* _multiplier (Variables|Default|GetGravity%20Mult)))
  (Variables|/Script/Engine.CharacterMovementComponent|SetMaxWalkSpeed _movement_comp_ref (/ (* (Variables|Default|GetSpeed%20Mult) (Variables|Default|GetMovement%20Speed)) _multiplier)))

(event Custom|Add%20Movement
  (params (scale :type Vector%202D%20Structure))
  (bind _returnvalue (Game|Player|GetPlayerPawn 0))
  (bind _returnvalue_2 (Pawn|GetControlRotation _returnvalue :!class /Script/Engine.Pawn))
  ;[1 1 1] Comment
  (Pawn|Input|AddMovementInput _returnvalue (Math|Vector|GetRightVector (Math|Rotator|MakeRotator (.roll _returnvalue_2) 0.0 (.yaw _returnvalue_2))) (.x scale) false)
  (Pawn|Input|AddMovementInput _returnvalue (Math|Vector|GetForwardVector (Math|Rotator|MakeRotator (.roll _returnvalue_2) 0.0 (.yaw _returnvalue_2))) (.y scale) false))

(event Input|EnhancedActionEvents|EnhancedInputActionIA_Move
  (params (ActionValue :type Vector%202D%20Structure) (ElapsedSeconds :type Float%20%28double-precision%29) (TriggeredSeconds :type Float%20%28double-precision%29) (InputAction :type Input%20Action%20Object%20Reference :default "/Game/Project_Modular_GBS/Blueprints/Player/Input/IA_Move.IA_Move"))
  ;[1 1 1] Comment
  (CallFunction|AddMovement ActionValue))

(event Input|EnhancedActionEvents|EnhancedInputActionIA_Look
  (params (ActionValue :type Vector%202D%20Structure) (ElapsedSeconds :type Float%20%28double-precision%29) (TriggeredSeconds :type Float%20%28double-precision%29) (InputAction :type Input%20Action%20Object%20Reference :default "/Game/Project_Modular_GBS/Blueprints/Player/Input/IA_Look.IA_Look"))
  ;[1 1 1] Comment
  (CallFunction|UpdateView ActionValue))

(event Input|EnhancedActionEvents|EnhancedInputActionIA_Run
  (params (ActionValue :type Vector%202D%20Structure) (ElapsedSeconds :type Float%20%28double-precision%29) (TriggeredSeconds :type Float%20%28double-precision%29) (InputAction :type Input%20Action%20Object%20Reference :default "/Game/Project_Modular_GBS/Blueprints/Player/Input/IA_Run.IA_Run"))
  (bind _movement_comp_ref (Variables|Default|GetMovement%20Comp%20Ref))
  ;[1 1 1] Comment
  (:Started
    (Variables|/Script/Engine.CharacterMovementComponent|SetMaxWalkSpeed _movement_comp_ref (Variables|Default|GetRun%20Speed)))
  (:Completed
    (Variables|/Script/Engine.CharacterMovementComponent|SetMaxWalkSpeed _movement_comp_ref (Variables|Default|GetMovement%20Speed))))

(event Input|EnhancedActionEvents|EnhancedInputActionIA_Use
  (params (ActionValue :type Boolean) (ElapsedSeconds :type Float%20%28double-precision%29) (TriggeredSeconds :type Float%20%28double-precision%29) (InputAction :type Input%20Action%20Object%20Reference :default "/Game/Project_Modular_GBS/Blueprints/Player/Input/IA_Use.IA_Use"))
  (bind _character_ref (Variables|Default|GetCharacter%20Ref))
  (bind _mesh (Variables|/Script/Engine.Character|GetMesh _character_ref))
  (bind _returnvalue (Components|SkeletalMesh|GetAnimInstance _mesh))
  ;[1 1 1] Comment
  (:Triggered
    (Variables|Default|SetFiring true)
    (CallFunction|LockRotation true)
    (Class|BPIAnimations|Firing(Message) _returnvalue true))
  (:Completed
    (Utilities|FlowControl|RetriggerableDelay 1.0)
    (Variables|Default|SetFiring false)
    (CallFunction|LockRotation false)
    (Class|BPIAnimations|Firing(Message) _returnvalue false)))

(event Input|EnhancedActionEvents|EnhancedInputActionIA_Aim
  (params (ActionValue :type Boolean) (ElapsedSeconds :type Float%20%28double-precision%29) (TriggeredSeconds :type Float%20%28double-precision%29) (InputAction :type Input%20Action%20Object%20Reference :default "/Game/Project_Modular_GBS/Blueprints/Player/Input/IA_Aim.IA_Aim"))
  (bind _character_ref (Variables|Default|GetCharacter%20Ref))
  (bind _mesh (Variables|/Script/Engine.Character|GetMesh _character_ref))
  (bind _returnvalue (Components|SkeletalMesh|GetAnimInstance _mesh))
  ;[1 1 1] Comment
  (:Started
    (Variables|Default|SetAiming true)
    (CallFunction|LockRotation true)
    (Class|BPIAnimations|Aiming(Message) _returnvalue true))
  (:Completed
    (Variables|Default|SetAiming false)
    (CallFunction|LockRotation false)
    (Class|BPIAnimations|Aiming(Message) _returnvalue false)))

(event Input|EnhancedActionEvents|EnhancedInputActionIA_Jump
  (params (ActionValue :type Boolean) (ElapsedSeconds :type Float%20%28double-precision%29) (TriggeredSeconds :type Float%20%28double-precision%29) (InputAction :type Input%20Action%20Object%20Reference :default "/Game/Project_Modular_GBS/Blueprints/Player/Input/IA_Jump.IA_Jump"))
  (bind _returnvalue (Game|GetPlayerCharacter 0))
  ;[1 1 1] Comment
  (:Started
    (Character|Jump _returnvalue))
  (:Completed
    (Character|StopJumping _returnvalue)))

(event Input|EnhancedActionEvents|EnhancedInputActionIA_Crouch
  (params (ActionValue :type Boolean) (ElapsedSeconds :type Float%20%28double-precision%29) (TriggeredSeconds :type Float%20%28double-precision%29) (InputAction :type Input%20Action%20Object%20Reference :default "/Game/Project_Modular_GBS/Blueprints/Player/Input/IA_Crouch.IA_Crouch"))
  (bind _character_ref (Variables|Default|GetCharacter%20Ref))
  ;[1 1 1] Comment
  (:Started
    (Character|Crouch _character_ref))
  (:Completed
    (Character|UnCrouch _character_ref)))

(event EventBeginPlay
  ;[1 1 1] Comment
  (bind _asplayer_controller (Utilities|Casting|CastToPlayerController (Pawn|GetController (Variables|/Script/Engine.Actor|GetInstigator (Components|GetOwner)))))
  (Utilities|IsValid (PlayerController|LocalPlayerSubsystems|GetEnhancedInputLocalPlayerSubsystem _asplayer_controller)
    (:Is%20Valid
      (Input|AddMappingContext (PlayerController|LocalPlayerSubsystems|GetEnhancedInputLocalPlayerSubsystem _asplayer_controller) "/Game/Project_Modular_GBS/Blueprints/Player/Input/IMC_Default.IMC_Default" 0 (Utilities|Struct|MakeModifyContextOptions true false false))
      (Variables|Default|SetMovement%20Comp%20Ref (Actor|GetComponentbyClass (Components|GetOwner) "/Script/Engine.CharacterMovementComponent"))
      (bind _ascharacter (Utilities|Casting|CastToCharacter (Components|GetOwner)))
      (Variables|Default|SetCharacter%20Ref _ascharacter)
      (bind _movement_comp_ref (Variables|Default|GetMovement%20Comp%20Ref)
        (:then
          (Variables|/Script/Engine.CharacterMovementComponent|SetMaxWalkSpeed _movement_comp_ref (Variables|Default|GetMovement%20Speed))
          (Variables|/Script/Engine.CharacterMovementComponent|SetGravityScale _movement_comp_ref (Variables|Default|GetGravity%20Mult)))
        (:else)))))

(event EventAdjustGravity
  (params (Precentage :type Float%20%28double-precision%29))
  (bind _returnvalue (Math|Float|Absolute(Float) Precentage))
  (bind _returnvalue_2 (/ _returnvalue 1e+02))
  ;[1 1 1] Comment
  ;;[1 1 1] Comment
  (if (> Precentage 0.0)
    (bind _output_get (Variables|Default|SetGravity%20Mult (* (stale _output_get) _returnvalue_2)))
    (else
      (bind _output_get_2 (Variables|Default|SetGravity%20Mult (/ (stale _output_get_2) _returnvalue_2)))))
  (CallFunction|TakeEffect))

(event EventAdjustSpeed
  (params (Precentage :type Float%20%28double-precision%29))
  (bind _returnvalue (Math|Float|Absolute(Float) Precentage))
  (bind _returnvalue_2 (/ _returnvalue 1e+02))
  ;[1 1 1] Comment
  ;;[1 1 1] Comment
  (if (> Precentage 0.0)
    (bind _output_get (Variables|Default|SetSpeed%20Mult (* (stale _output_get) _returnvalue_2)))
    (else
      (bind _output_get_2 (Variables|Default|SetSpeed%20Mult (/ (stale _output_get_2) _returnvalue_2)))))
  (CallFunction|TakeEffect))

(event EventAdjustWeight
  (params (Amount%20KG :type Float%20%28double-precision%29))
  ;[1 1 1] Comment
  ;;[1 1 1] Comment
  (bind _output_get (Variables|Default|SetAdditional%20Weight (+ (stale _output_get) Amount%20KG)))
  (CallFunction|TakeEffect))

(fn LockRotation
  (params (On/Off :type Boolean))
  (bind _returnvalue (not On/Off))
  (bind _movement_comp_ref (Variables|Default|GetMovement%20Comp%20Ref))
  ;[1 1 1] Comment
  (if (not (and _returnvalue (or (Variables|Default|GetAiming) (Variables|Default|GetFiring))))
    (Variables|/Script/Engine.CharacterMovementComponent|SetRotationRate _movement_comp_ref (Math|Rotator|MakeRotator 0.0 0.0 (Math|Float|SelectFloat 3.6e+02 7.2e+02 On/Off)))
    (bind _output_get (Variables|/Script/Engine.CharacterMovementComponent|SetbOrientRotationToMovement _movement_comp_ref _returnvalue))
    (Variables|/Script/Engine.CharacterMovementComponent|SetbUseControllerDesiredRotation _movement_comp_ref (not _output_get))
    (return)))