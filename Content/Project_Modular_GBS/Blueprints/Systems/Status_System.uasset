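; Status component that tracks one attribute, such as Health or Shield, on its owning actor and can regenerate it.
; Adjustments clamp the value between zero and max, report any overflow, and push updates to the owner's name-system 3D widget and a W_Main bar.
; TryAdjust also starts a delayed, timer-driven regeneration that steps toward max.
; The screen bar binds only for PlayerController-driven characters, despite the check being named IsPlayerAnAI.
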(event Custom|Try%20Regeneration
  (if (Variables|Settings|GetRegeneration)
    (Utilities|Time|SetTimerbyEvent (EventDispatchers|CreateEvent :!event RegenerateLoop) (Variables|Settings|GetRegeneration%20Delay))))

(event EventBeginPlay
  (bind _max_value (Variables|Settings|GetMax_Value))
  (bind _current_value (Variables|Settings|GetCurrent_Value))
  (bind _status_attribute (Variables|Settings|GetStatus%20Attribute))
  (Utilities|FlowControl|Delay 0.2)
  (if (CallFunction|IsPlayerAnAI (Components|GetOwner))
    (CallFunction|GetScreenWidget))
  (CallFunction|Get3DWidget)
  (Class|BPIStatus|AdjustStatus(Message) (Variables|Default|GetWidget%20Ref) _status_attribute false _current_value _max_value)
  (Class|BPIStatus|AdjustStatus(Message) (Variables|Default|Get3D%20Widget%20Ref) _status_attribute false _current_value _max_value))

(event EventAdjustStatus
  (params (Target%20Stat :type E_Status%20Enum :default "NewEnumerator3") (Add/Remove :type Boolean) (Value :type Float%20%28double-precision%29) (Max%20Value :type Float%20%28double-precision%29) (Causer :type Actor%20Object%20Reference))
  (CallFunction|TryAdjust Add/Remove Value))

(fn GetScreenWidget
  (bind _foundwidgets (Widget|GetAllWidgetsOfClass "/Game/Project_Modular_GBS/Default_Demo_Widgets/W_Main.W_Main_C" false))
  (Utilities|IsValid (Utilities|Array|Get(acopy) _foundwidgets)
    (:Is%20Valid
      (switch Utilities|FlowControl|Switch|SwitchonE_Status (Variables|Settings|GetStatus%20Attribute)
        (:NewEnumerator0
          (Variables|Default|SetWidget%20Ref (Variables|/Game/Project_Modular_GBS/Default_Demo_Widgets/W_Main.W_Main_C|GetW_Health_Bar (Utilities|Array|Get(acopy) _foundwidgets))))
        (:NewEnumerator1
          (Variables|Default|SetWidget%20Ref (Variables|/Game/Project_Modular_GBS/Default_Demo_Widgets/W_Main.W_Main_C|GetW_Shield_Bar (Utilities|Array|Get(acopy) _foundwidgets))))))))

(fn Get3DWidget
  (bind _returnvalue (Components|GetOwner))
  (bind _returnvalue_2 (Actor|GetComponentbyClass _returnvalue "/Game/Project_Modular_GBS/Blueprints/Systems/Player_Name_System.Player_Name_System_C"))
  (Utilities|IsValid _returnvalue_2
    (:Is%20Valid
      (Variables|Default|Set3D%20Widget%20Ref (Variables|/Game/Project_Modular_GBS/Blueprints/Systems/Player_Name_System.Player_Name_System_C|GetWidget%20Ref _returnvalue_2)))))

(fn DirectAdjust
  (params (Add/Remove :type Boolean) (Value :type Float%20%28double-precision%29))
  (bind _returnvalue (Math|Float|Absolute(Float) Value))
  (bind _max_value (Variables|Settings|GetMax_Value))
  (bind _status_attribute (Variables|Settings|GetStatus%20Attribute))
  (LocalVariables|SetAmount%201 (Math|Float|Absolute(Float) (- (+ (Variables|Settings|GetCurrent_Value) (Math|Float|SelectFloat _returnvalue (* _returnvalue -1.0) Add/Remove)) (Math|Float|Clamp(Float) (+ (Variables|Settings|GetCurrent_Value) (Math|Float|SelectFloat _returnvalue (* _returnvalue -1.0) Add/Remove)) 0.0 _max_value))))
  (LocalVariables|SetOut%20of%20Range%201 (or (> (+ (Variables|Settings|GetCurrent_Value) (Math|Float|SelectFloat _returnvalue (* _returnvalue -1.0) Add/Remove)) (Math|Float|Clamp(Float) (+ (Variables|Settings|GetCurrent_Value) (Math|Float|SelectFloat _returnvalue (* _returnvalue -1.0) Add/Remove)) 0.0 _max_value)) (< (+ (Variables|Settings|GetCurrent_Value) (Math|Float|SelectFloat _returnvalue (* _returnvalue -1.0) Add/Remove)) (Math|Float|Clamp(Float) (+ (Variables|Settings|GetCurrent_Value) (Math|Float|SelectFloat _returnvalue (* _returnvalue -1.0) Add/Remove)) 0.0 _max_value))))
  (bind _output_get (Variables|Settings|SetCurrent_Value (Math|Float|Clamp(Float) (+ (Variables|Settings|GetCurrent_Value) (Math|Float|SelectFloat _returnvalue (* _returnvalue -1.0) Add/Remove)) 0.0 _max_value)))
  (Class|BPIStatus|AdjustStatus(Message) (Variables|Default|GetWidget%20Ref) _status_attribute false _output_get _max_value)
  (Class|BPIStatus|AdjustStatus(Message) (Variables|Default|Get3D%20Widget%20Ref) _status_attribute false _output_get _max_value)
  (return (LocalVariables|GetOut%20of%20Range%201) (LocalVariables|GetAmount%201)))

(fn IsPlayerAnAI
  (params (Owner :type Object%20Object%20Reference))
  (bind _ascharacter (Utilities|Casting|CastToCharacter Owner)
    (:then
      (Utilities|Casting|CastToPlayerController (Pawn|GetController _ascharacter)
        (:then
          (return true))
        (:CastFailed
          _)))
    (:CastFailed
      _))
  (return false))

(fn RegenerateLoop
  (if (Variables|Settings|GetRegeneration)
    (if (== (Variables|Settings|GetCurrent_Value) (Variables|Settings|GetMax_Value))
      (Development|PrintString "End")
      (else
        (CallFunction|DirectAdjust true (Variables|Settings|GetRegeneration%20Amount))
        (Utilities|Time|SetTimerbyEvent (EventDispatchers|CreateEvent :!event RegenerateLoop) (/ 1.0 (Variables|Settings|GetRegeneration%20Speed)))))))

(fn TryAdjust
  (params (Add/Remove :type Boolean) (Value :type Float%20%28double-precision%29))
  (bind (_out_of_range _amount) (CallFunction|DirectAdjust Add/Remove Value))
  (CallFunction|TryRegeneration)
  (return _out_of_range _amount))