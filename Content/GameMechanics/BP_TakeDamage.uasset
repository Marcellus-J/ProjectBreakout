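; BP_TakeDamage is a damage-handling Blueprint that subtracts incoming damage from Health and prints the remaining value.
; At zero or below, it attempts a ragdoll death by enabling physics simulation, full blend weight and collision on a skeletal mesh.
; That mesh comes from casting player 0's pawn, rather than its component, to SkeletalMeshComponent, so the cast fails and the ragdoll never runs.
; Leftover DefaultPawn casts are unconnected.
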(event Custom|TakeDamage
  (params (Damage :type Float%20%28single-precision%29) (DamageType :type Damage%20Type%20Object%20Reference) (InstigatedBy :type Controller%20Object%20Reference) (DamageCauser :type Actor%20Object%20Reference))
  ;[1 1 1] Take Damage
  (if (> (Variables|Default|GetHealth) 0.0)
    (bind _output_get (Variables|Default|SetHealth (- (Variables|Default|GetHealth) Damage)))
    (Development|PrintString (Utilities|String|ToString(Float) _output_get))
    (if (<= (Variables|Default|GetHealth) 0.0)
      (bind _asskeletal_mesh_component (Utilities|Casting|CastToSkeletalMeshComponent (Game|Player|GetPlayerPawn 0)))
      (Physics|SetSimulatePhysics _asskeletal_mesh_component true)
      (Class|SkeletalMeshComponent|SetPhysicsBlendWeight _asskeletal_mesh_component 1.0)
      (Collision|SetCollisionEnabled _asskeletal_mesh_component "QueryAndPhysics"))))

(event EventTick
  (params (DeltaSeconds :type Float%20%28single-precision%29)))

(event EventBeginPlay)